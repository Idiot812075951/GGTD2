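; BP_Player is the player character Blueprint, driving attributes and skills through the Gameplay Ability System.
; After a short delay on BeginPlay, it applies GE_InitAttribute to its ability system component.
; Fire and Dragon events each grant and activate their fireball or dragon-range ability once, while PrintHp prints base and current Health for debugging.
; The Q and E skill inputs, overlap and Tick events are empty.
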(event Custom|Fire
  (Class|AbilitySystemComponent|GiveAbilityandActivateOnce (Variables|Default|GetAsc) "/Game/GGTD/GAS/GA/FireBall/GA_FireBall_BP.GA_FireBall_BP_C" 0 -1))

(event Custom|Dragon
  (Class|AbilitySystemComponent|GiveAbilityandActivateOnce (Variables|Default|GetAsc) "/Game/GGTD/GAS/GA/DragonRage/GA_DragonRange_BP.GA_DragonRange_BP_C" 0 -1))

(event Custom|PrintHp
  (bind _returnvalue (GameplayAttributes|GetAttributeSet (Variables|Default|GetAsc) "/Script/GGTD2.GGTD2_AttributeSet"))
  (Utilities|IsValid _returnvalue
    (:Is%20Valid
      (Development|PrintString (Utilities|String|ToString(Float) (.BaseValue (Utilities|Struct|BreakGameplayAttributeData (Variables|/Script/GGTD2.GGTD2_AttributeSet|GetHealth _returnvalue)))))
      (Development|PrintString (Utilities|String|ToString(Float) (.CurrentValue (Utilities|Struct|BreakGameplayAttributeData (Variables|/Script/GGTD2.GGTD2_AttributeSet|GetHealth _returnvalue))))))
    (:Is%20Not%20Valid
      (Development|PrintString "属性集空了"))))

(event Input|EnhancedActionEvents|EnhancedInputActionIA_SkillQ
  (params (ActionValue :type Boolean) (ElapsedSeconds :type Float%20%28double-precision%29) (TriggeredSeconds :type Float%20%28double-precision%29) (InputAction :type Input%20Action%20Object%20Reference :default "/Game/TopDown/Input/Actions/IA_SkillQ.IA_SkillQ")))

(event Input|EnhancedActionEvents|EnhancedInputActionIA_SkillE
  (params (ActionValue :type Boolean) (ElapsedSeconds :type Float%20%28double-precision%29) (TriggeredSeconds :type Float%20%28double-precision%29) (InputAction :type Input%20Action%20Object%20Reference :default "/Game/TopDown/Input/Actions/IA_SkillE.IA_SkillE")))

(event Collision|EventActorBeginOverlap
  (params (OtherActor :type Actor%20Object%20Reference)))

(event EventTick
  (params (DeltaSeconds :type Float%20%28single-precision%29)))

(event EventBeginPlay
  (Utilities|FlowControl|Delay 2.0)
  (GameplayEffects|ApplyGameplayEffectToSelf :self (Variables|Default|GetAsc) :GameplayEffectClass "/Game/GGTD/GAS/GE/GE_InitAttribute.GE_InitAttribute_C"))

(event Input|KeyboardEvents|DebugKey1
  (params (Key :type Key%20Structure :default "None") (ActionValue :type Input%20Action%20Value%20Structure)))

(fn ConstructionScript)
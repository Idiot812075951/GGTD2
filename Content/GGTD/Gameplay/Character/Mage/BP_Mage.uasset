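; Mage player character that uses the Gameplay Ability System for its skills and has a key-triggered knockback.
; After a startup delay it applies initial attributes and spawns a physics constraint actor; Q and E grant-and-activate Fireball and Dragon Rage abilities.
; Key 3 sphere-traces for a nearby character, temporarily simulates physics on its capsule and launches it forward and up.
; During the launch, a constraint to the Mage's capsule locks twist and Swing2 while leaving linear motion free.
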(event Custom|DragonRage
  (Class|AbilitySystemComponent|GiveAbilityandActivateOnce (Variables|Default|GetAsc) "/Game/GGTD/GAS/GA/DragonRage/GA_DragonRange_BP.GA_DragonRange_BP_C" 0 -1))

(event Custom|Impulse
  (params (TargetCharacter :type Character%20Object%20Reference))
  (bind _self self)
  (bind _capsulecomponent (Variables|/Script/Engine.Character|GetCapsuleComponent TargetCharacter))
  (bind _physicsconstraintactor (Variables|Default|GetPhysicsConstraintActor))
  (bind _constraintcomp (Variables|/Script/Engine.PhysicsConstraintActor|GetConstraintComp _physicsconstraintactor))
  (if (Utilities|IsValid (Variables|Default|GetPhysicsConstraintActor))
    (Transformation|SetActorLocation (Variables|Default|GetPhysicsConstraintActor) (+ (Transformation|GetActorLocation _self) (* (Transformation|GetActorForwardVector _self) "10.000000,10.000000,10.000000")) true false)
    (Physics|SetSimulatePhysics _capsulecomponent true)
    (Class|PhysicsConstraintComponent|SetConstrainedComponents _constraintcomp (Variables|Default|GetCapsuleComponent) "None" _capsulecomponent "None")
    (Class|PhysicsConstraintComponent|SetAngularSwing2Limit _constraintcomp "ACM_Locked" 0.0)
    (Class|PhysicsConstraintComponent|SetAngularTwistLimit _constraintcomp "ACM_Locked" 0.0)
    (Class|PhysicsConstraintComponent|SetLinearXLimit _constraintcomp "LCM_Free" 0.0)
    (Class|PhysicsConstraintComponent|SetLinearYLimit _constraintcomp "LCM_Free" 0.0)
    (Class|PhysicsConstraintComponent|SetLinearZLimit _constraintcomp "LCM_Free" 0.0)
    (Utilities|FlowControl|DelayUntilNextTick)
    (Physics|AddImpulse _capsulecomponent (+ (* (Transformation|GetActorForwardVector self) 1e+03) "0.000000,0.000000,500.000000") "None" true)
    (Utilities|FlowControl|Delay 1.8)
    (Physics|SetSimulatePhysics _capsulecomponent false)
    (Class|PhysicsConstraintComponent|BreakConstraint (Variables|/Script/Engine.PhysicsConstraintActor|GetConstraintComp (Variables|Default|GetPhysicsConstraintActor)))
    (else
      (Development|PrintString "PhysicsConstraintActor 空了"))))

(event Custom|FireBall
  (Class|AbilitySystemComponent|GiveAbilityandActivateOnce (Variables|Default|GetAsc) "/Game/GGTD/GAS/GA/FireBall/GA_NewFireBall_BP.GA_NewFireBall_BP_C" 0 -1))

(event Input|EnhancedActionEvents|EnhancedInputActionIA_SkillQ
  (params (ActionValue :type Boolean) (ElapsedSeconds :type Float%20%28double-precision%29) (TriggeredSeconds :type Float%20%28double-precision%29) (InputAction :type Input%20Action%20Object%20Reference :default "/Game/TopDown/Input/Actions/IA_SkillQ.IA_SkillQ"))
  (:Completed
    (CallFunction|FireBall)))

(event Input|EnhancedActionEvents|EnhancedInputActionIA_SkillE
  (params (ActionValue :type Boolean) (ElapsedSeconds :type Float%20%28double-precision%29) (TriggeredSeconds :type Float%20%28double-precision%29) (InputAction :type Input%20Action%20Object%20Reference :default "/Game/TopDown/Input/Actions/IA_SkillE.IA_SkillE"))
  (:Completed
    (CallFunction|DragonRage)))

(event Collision|EventActorBeginOverlap
  (params (OtherActor :type Actor%20Object%20Reference)))

(event EventTick
  (params (DeltaSeconds :type Float%20%28single-precision%29)))

(event EventBeginPlay
  (Utilities|FlowControl|Delay 2.0)
  (GameplayEffects|ApplyGameplayEffectToSelf :self (Variables|Default|GetAsc) :GameplayEffectClass "/Game/GGTD/GAS/GE/GE_InitAttribute.GE_InitAttribute_C")
  (bind _returnvalue (Game|SpawnActorfromClass "/Script/Engine.PhysicsConstraintActor" (Transformation|GetActorTransform) "Undefined" "MultiplyWithRoot" 0 0))
  (Variables|Default|SetPhysicsConstraintActor _returnvalue))

(event Input|KeyboardEvents|1
  (params (Key :type Key%20Structure :default "None")))

(event Input|KeyboardEvents|3
  (params (Key :type Key%20Structure :default "None"))
  (:Pressed
    (bind (_targetcharacter _isfind) (CallFunction|FindTargetCharacterbyRadius 1e+03 (Variables|Default|GetObject%20Type%20Query)))
    (if _isfind
      (CallFunction|Impulse _targetcharacter))))

(fn ConstructionScript)

(fn FindTargetCharacterbyRadius
  (params (Radius :type Float%20%28double-precision%29) (ObjectTypeQuery :type Array%20of%20EObjectTypeQuery%20Enums :default "ObjectTypeQuery1"))
  (bind _self self)
  (bind _returnvalue (Transformation|GetActorLocation _self))
  (bind (_outhits _returnvalue_2) (Collision|MultiSphereTraceForObjects _returnvalue _returnvalue Radius ObjectTypeQuery false 0 "ForDuration"))
  (if _returnvalue_2
    (bind _ascharacter (Utilities|Casting|CastToCharacter (.HitActor (Collision|BreakHitResult (Utilities|Array|Get(acopy) _outhits))))
      (:then
        (Development|PrintString (Utilities|GetDisplayName (.HitActor (Collision|BreakHitResult (Utilities|Array|Get(acopy) _outhits)))))
        (return _ascharacter true))
      (:CastFailed
        _)))
  (return 0 false))